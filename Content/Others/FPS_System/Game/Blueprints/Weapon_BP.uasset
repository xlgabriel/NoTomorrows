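; Weapon Blueprint for an FPS, handling firing, fire modes, reloading and weapon switching for the player.
; Fire runs auto, burst or single-shot macros that play montages; each shot deducts ammo and calls Projectile, then reloads or switches when empty.
; Projectile adds recoil, effects and shake, spawns a bullet, and line-traces from the camera with movement-based spread to place impacts.
; Reload picks short or long animations, and switching swaps inventory weapons between hand and holster sockets.
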(event `self.ReceiveBeginPlay`
  ;[1 1 1] Event Begin Play
  (set `self.HasFireModes` (`.FireModes_37_28A161AE45D893CA1E63A4997466354B` (break `/Game/Others/FPS_System/Game/Blueprints/Weapon_Struct` (`self.WeaponData`)))))

(event `SingleShot`
  ;[1 1 1] Animations
  ;;[1 1 1] Shot Montages
  (bind _mesh (`self.Cast to Player`))
  (bind _output_get (set `self.OneShot` (`self.OneShot`)))
  (`|PlayMontage` _mesh _output_get))

(event `Aim_SingleShot`
  ;[1 1 1] Animations
  ;;[1 1 1] Aim Shot Montages
  (bind _mesh (`self.Cast to Player`))
  (bind _output_get (set `self.Aim_OneShot` (`self.Aim_OneShot`)))
  (`|PlayMontage` _mesh _output_get))

(event `Weapon_SingleShot`
  ;[1 1 1] Animations
  ;;[1 1 1] Weapon Shot Montages
  (bind _output_get (set `self.Weapon_OneShot` (`self.Weapon_OneShot`)))
  (`SkeletalMeshComponent.PlayAnimation` (`self.WeaponMesh`) _output_get false))

(event `FireMode`
  ;[1 1 1] FireMode
  (if (`.FireModes_37_28A161AE45D893CA1E63A4997466354B` (break `/Game/Others/FPS_System/Game/Blueprints/Weapon_Struct` (`self.WeaponData`)))
    (switch `/Game/Others/FPS_System/Game/Blueprints/FireMode_Enum` (`self.FireModes`)
      (:`NewEnumerator0`
        (set `self.FireModes` "NewEnumerator1"))
      (:`NewEnumerator1`
        (set `self.FireModes` "NewEnumerator2"))
      (:`NewEnumerator2`
        (set `self.FireModes` "NewEnumerator0")))))

(event `MultipleShots`
  ;[1 1 1] Animations
  ;;[1 1 1] Shot Montages
  (bind _mesh (`self.Cast to Player`))
  (bind _output_get (set `self.MultiShot` (`self.MultiShot`)))
  (`|PlayMontage` _mesh _output_get))

(event `Aim_MultipleShots`
  ;[1 1 1] Animations
  ;;[1 1 1] Aim Shot Montages
  (bind _mesh (`self.Cast to Player`))
  (bind _output_get (set `self.Aim_MultiShot` (`self.Aim_MultiShot`)))
  (`|PlayMontage` _mesh _output_get))

(event `Weapon_MultipleShots`
  ;[1 1 1] Animations
  ;;[1 1 1] Weapon Shot Montages
  (bind _output_get (set `self.Weapon_MultiShot` (`self.Weapon_MultiShot`)))
  (`SkeletalMeshComponent.PlayAnimation` (`self.WeaponMesh`) _output_get false))

(event `NoFire`
  (bind _returnvalue (`GameplayStatics.GetPlayerCharacter` 0))
  (bind _weapondata (`self.WeaponData`))
  (bind _weapondata_2 (`self.WeaponData`))
  ;[1 1 1] Fire
  ;;[1 1 1] Auto
  (`|ExecutionSequence`
    (:`then_0`
      (`Character.StopAnimMontage` _returnvalue (`self.Aim_MultiShot`))
      (goto _label :!via `Close`))
    (:`then_1`
      (`Character.StopAnimMontage` _returnvalue (`self.MultiShot`))
      (goto _label :!via `Close`))
    (:`then_2`
      (`AnimInstance.Montage_Stop` (`SkeletalMeshComponent.GetAnimInstance` (`self.WeaponMesh`)) 0.3 (`self.Weapon_MultiShot`)))))

(event `Reload_Short`
  ;[1 1 1] Animations
  ;;[1 1 1] Reload Short Montage
  (`|ExecutionSequence`
    (:`then_0`
      (bind _mesh (`self.Cast to Player`))
      (bind _output_get (set `self.ReloadShort` (`self.ReloadShort`)))
      (`|PlayMontage` _mesh _output_get))
    (:`then_1`
      (bind _output_get_2 (set `self.Weapon_ReloadShort` (`self.Weapon_ReloadShort`)))
      (`SkeletalMeshComponent.PlayAnimation` (`self.WeaponMesh`) _output_get_2 false))))

(event `Reload_Long`
  ;[1 1 1] Animations
  ;;[1 1 1] Reload Long Montage
  (`|ExecutionSequence`
    (:`then_0`
      (bind _mesh (`self.Cast to Player`))
      (bind _output_get (set `self.ReloadLong` (`self.ReloadLong`)))
      (`|PlayMontage` _mesh _output_get))
    (:`then_1`
      (bind _output_get_2 (set `self.Weapon_ReloadLong` (`self.Weapon_ReloadLong`)))
      (`SkeletalMeshComponent.PlayAnimation` (`self.WeaponMesh`) _output_get_2 false))))

(event `Fire`
  (bind _returnvalue (`GameplayStatics.GetPlayerCharacter` 0))
  (bind _weapondata (`self.WeaponData`))
  (bind _weapondata_2 (`self.WeaponData`))
  ;[1 1 1] Fire
  (if (not (or (`self.IsSwitching`) (`self.IsReloading`)))
    (`self.AmmoCheck`)
    (set `self.IsShooting` true)
    (if (`self.HasFireModes`)
      (switch `/Game/Others/FPS_System/Game/Blueprints/FireMode_Enum` (`self.FireModes`)
        (:`NewEnumerator0`
          (set `self.IsAuto` true)
          ;;[1 1 1] Auto
          (`self.Weapon_MultipleShots`)
          (bind _asplayer_bp (cast `/Game/Others/FPS_System/Game/Blueprints/Player_BP` (`GameplayStatics.GetPlayerCharacter` 0)))
          (if (`/Game/Others/FPS_System/Game/Blueprints/Player_BP.IsAiming` _asplayer_bp)
            (`self.Aim_MultipleShots`)
            (else
              (`self.MultipleShots`)))
          (`|ExecutionSequence`
            (:`then_0`
              (goto _label :!via `Open`))
            (:`then_1`
              (`/Engine/EditorBlueprintResources/StandardMacros.Gate` true :!label _label
                (:`Exit`
                  (`|ExecutionSequence`
                    (:`then_0`
                      (setmembers `/Game/Others/FPS_System/Game/Blueprints/Weapon_Struct` :`StructRef` _weapondata :`CurrentAmmo` (- (`.CurrentAmmo_45_1757189B473A397F6343EB94A3EE76E9` (break `/Game/Others/FPS_System/Game/Blueprints/Weapon_Struct` _weapondata)) 1) :!label _label_2)
                      (`self.Projectile`)
                      (set `self.IsShooting` false)
                      (if (== (`.CurrentAmmo_45_1757189B473A397F6343EB94A3EE76E9` (break `/Game/Others/FPS_System/Game/Blueprints/Weapon_Struct` _weapondata_2)) 0)
                        (if (== (`.MaxAmmo_46_0B4159594B8BAC470906F2A0EFE95895` (break `/Game/Others/FPS_System/Game/Blueprints/Weapon_Struct` _weapondata_2)) 0)
                          (`self.Empty`)
                          (`KismetSystemLibrary.Delay` 0.2)
                          (`self.SwitchWeapons`)
                          (else
                            (`self.Reload`)))))
                    (:`then_1`
                      (`self.AmmoCheck`)
                      (if (not (or (`self.IsSwitching`) (`self.IsReloading`)))
                        (`KismetSystemLibrary.RetriggerableDelay` (`.FireRate_32_9CE1D5284CA4F884888B57A5CCD44BE9` (break `/Game/Others/FPS_System/Game/Blueprints/Weapon_Struct` (`self.WeaponData`))))
                        (goto _label)))))))))
        (:`NewEnumerator1`
          (set `self.IsAuto` false)
          ;;[1 1 1] Burst
          (`self.Weapon_MultipleShots`)
          (bind _asplayer_bp_2 (cast `/Game/Others/FPS_System/Game/Blueprints/Player_BP` (`GameplayStatics.GetPlayerCharacter` 0)))
          (if (`/Game/Others/FPS_System/Game/Blueprints/Player_BP.IsAiming` _asplayer_bp_2)
            (`self.Aim_MultipleShots`)
            (else
              (`self.MultipleShots`)))
          (`|ExecutionSequence`
            (:`then_0`
              (goto _label_3 :!via `Open`))
            (:`then_1`
              (`/Engine/EditorBlueprintResources/StandardMacros.Gate` true :!label _label_3
                (:`Exit`
                  (`|ExecutionSequence`
                    (:`then_0`
                      (`/Engine/EditorBlueprintResources/StandardMacros.Do N` 3 :!label _label_4
                        (:`Exit`
                          (`self.AmmoCheck`)
                          (`|ExecutionSequence`
                            (:`then_0`
                              (goto _label_2))
                            (:`then_1`
                              (`KismetSystemLibrary.Delay` 0.3)
                              (if (`/Game/Others/FPS_System/Game/Blueprints/Player_BP.IsAiming` _asplayer_bp_2)
                                (`Character.StopAnimMontage` _returnvalue (`self.Aim_MultiShot`))
                                (else
                                  (`Character.StopAnimMontage` _returnvalue (`self.MultiShot`))))
                              (`AnimInstance.Montage_Stop` (`SkeletalMeshComponent.GetAnimInstance` (`self.WeaponMesh`)) 0.3 (`self.Weapon_MultiShot`)))))))
                    (:`then_1`
                      (`KismetSystemLibrary.RetriggerableDelay` 0.07)
                      (goto _label_3))
                    (:`then_2`
                      (`KismetSystemLibrary.Delay` 0.5)
                      (goto _label_4 :!via `Reset`))))))
            (:`then_2`
              (`KismetSystemLibrary.Delay` 0.3)
              (goto _label_3 :!via `Close`))))
        (:`NewEnumerator2`
          (set `self.IsAuto` false)
          ;;[1 1 1] Single
          (`self.Weapon_SingleShot` :!label _label_5)
          (bind _asplayer_bp_3 (cast `/Game/Others/FPS_System/Game/Blueprints/Player_BP` (`GameplayStatics.GetPlayerCharacter` 0)))
          (if (`/Game/Others/FPS_System/Game/Blueprints/Player_BP.IsAiming` _asplayer_bp_3)
            (`self.Aim_SingleShot`)
            (else
              (`self.SingleShot`)))
          (`self.AmmoCheck`)
          (`|ExecutionSequence`
            (:`then_0`
              (goto _label_2))
            (:`then_1`
              (`KismetSystemLibrary.Delay` 0.2)
              (`Character.StopAnimMontage` (`GameplayStatics.GetPlayerCharacter` 0) (`self.OneShot`))))))
      (else
        (goto _label_5)))))

(event `Empty`
  ;[1 1 1] Animations
  ;;[1 1 1] Empty
  (`SkeletalMeshComponent.PlayAnimation` (`self.WeaponMesh`) "/Game/Others/FPS_System/Game/Weapons/Pistol/Animations/Pistol/Pistol_Empty.Pistol_Empty" false))

(event `Reload`
  (bind _neededammo (`self.NeededAmmo`))
  (bind _weapondata (`self.WeaponData`))
  (bind _weapondata_2 (`self.WeaponData`))
  (bind _weapondata_3 (`self.WeaponData`))
  (bind ((`MagazineSize_7_76E520B34EC71DF016211C9907BE14D7` _magazinesize) (`CurrentAmmo_45_1757189B473A397F6343EB94A3EE76E9` _currentammo)) (break `/Game/Others/FPS_System/Game/Blueprints/Weapon_Struct` (`self.WeaponData`)))
  (bind ((`MagazineSize_7_76E520B34EC71DF016211C9907BE14D7` _magazinesize_2) (`CurrentAmmo_45_1757189B473A397F6343EB94A3EE76E9` _currentammo_2)) (break `/Game/Others/FPS_System/Game/Blueprints/Weapon_Struct` (`self.WeaponData`)))
  (bind ((`CurrentAmmo_45_1757189B473A397F6343EB94A3EE76E9` _currentammo_3) (`MaxAmmo_46_0B4159594B8BAC470906F2A0EFE95895` _maxammo)) (break `/Game/Others/FPS_System/Game/Blueprints/Weapon_Struct` (`self.WeaponData`)))
  (bind ((`MaxAmmo_46_0B4159594B8BAC470906F2A0EFE95895` _maxammo_2)) (break `/Game/Others/FPS_System/Game/Blueprints/Weapon_Struct` (`self.WeaponData`)))
  (bind ((`MagazineSize_7_76E520B34EC71DF016211C9907BE14D7` _magazinesize_3) (`MaxAmmo_46_0B4159594B8BAC470906F2A0EFE95895` _maxammo_3)) (break `/Game/Others/FPS_System/Game/Blueprints/Weapon_Struct` _weapondata_3))
  (bind _returnvalue (- _maxammo_2 _neededammo))
  ;[1 1 1] Reload
  (`/Engine/EditorBlueprintResources/StandardMacros.DoOnce` false :!label _label_6
    (:`Completed`
      (if (> (`.MaxAmmo_46_0B4159594B8BAC470906F2A0EFE95895` (break `/Game/Others/FPS_System/Game/Blueprints/Weapon_Struct` (`self.WeaponData`))) 0)
        (if (not (== (+ _magazinesize_2 1) _currentammo_2))
          (set `self.IsReloading` true)
          (set `self.NeededAmmo` (- _magazinesize _currentammo))
          (if (<= _maxammo_2 _neededammo)
            (`self.Reload_Long`)
            (`KismetSystemLibrary.Delay` (`.ReloadLong_Length_58_65EFE1A6436BB6ECDBAB14964D76A4D0` (break `/Game/Others/FPS_System/Game/Blueprints/Weapon_Struct` (`self.WeaponData`))))
            (setmembers `/Game/Others/FPS_System/Game/Blueprints/Weapon_Struct` :`StructRef` _weapondata_2 :`CurrentAmmo` (+ _currentammo_3 _maxammo))
            (setmembers `/Game/Others/FPS_System/Game/Blueprints/Weapon_Struct` :`StructRef` _weapondata_2 :`MaxAmmo` 0)
            (set `self.IsReloading` false)
            (goto _label_6 :!via `Reset`)
            (elif (> (`.CurrentAmmo_45_1757189B473A397F6343EB94A3EE76E9` (break `/Game/Others/FPS_System/Game/Blueprints/Weapon_Struct` (`self.WeaponData`))) 0)
              (`self.Reload_Short`)
              (`KismetSystemLibrary.Delay` (`.ReloadShort_Length_59_40885D4B4F95B1004C1E1298A4E40D11` (break `/Game/Others/FPS_System/Game/Blueprints/Weapon_Struct` _weapondata)))
              (setmembers `/Game/Others/FPS_System/Game/Blueprints/Weapon_Struct` :`StructRef` _weapondata_3 :`MaxAmmo` _returnvalue)
              (setmembers `/Game/Others/FPS_System/Game/Blueprints/Weapon_Struct` :`StructRef` _weapondata_3 :`CurrentAmmo` (+ _magazinesize_3 1))
              (setmembers `/Game/Others/FPS_System/Game/Blueprints/Weapon_Struct` :`StructRef` _weapondata_3 :`MaxAmmo` (- _maxammo_3 1))
              (set `self.IsReloading` false)
              (goto _label_6 :!via `Reset`)
              (else
                (`self.Reload_Long`)
                (`KismetSystemLibrary.Delay` (`.ReloadLong_Length_58_65EFE1A6436BB6ECDBAB14964D76A4D0` (break `/Game/Others/FPS_System/Game/Blueprints/Weapon_Struct` _weapondata)))
                (setmembers `/Game/Others/FPS_System/Game/Blueprints/Weapon_Struct` :`StructRef` _weapondata_3 :`MaxAmmo` _returnvalue)
                (setmembers `/Game/Others/FPS_System/Game/Blueprints/Weapon_Struct` :`StructRef` _weapondata_3 :`CurrentAmmo` (`.MagazineSize_7_76E520B34EC71DF016211C9907BE14D7` (break `/Game/Others/FPS_System/Game/Blueprints/Weapon_Struct` (`self.WeaponData`))))
                (set `self.IsReloading` false)
                (goto _label_6 :!via `Reset`)))))
        (else
          (goto _label_6 :!via `Reset`))))))

(event `SwitchWeapons`
  (bind _playerref (`self.PlayerRef`))
  (bind _playerref_2 (`self.PlayerRef`))
  (bind _playerref_3 (`self.PlayerRef`))
  (bind _output (`|GetArrayItem` (`/Game/Others/FPS_System/Game/Blueprints/Player_BP.WeaponInventory` _playerref_3) (`/Game/Others/FPS_System/Game/Blueprints/Player_BP.WeaponIndex` _playerref_3)))
  (bind _output_2 (`|GetArrayItem` (`/Game/Others/FPS_System/Game/Blueprints/Player_BP.WeaponInventory` _playerref_2) (`/Game/Others/FPS_System/Game/Blueprints/Player_BP.WeaponIndex` _playerref_2)))
  ;[1 1 1] Switch Weapons
  (set `self.IsSwitching` true)
  (bind (_mesh _playerref_4) (`self.Cast to Player`))
  (`|ExecutionSequence`
    (:`then_0`
      (bind _returnvalue (+ (`/Game/Others/FPS_System/Game/Blueprints/Player_BP.WeaponIndex` _playerref_4) 1))
      (if (> _returnvalue (- (`KismetArrayLibrary.Array_Length` (`/Game/Others/FPS_System/Game/Blueprints/Player_BP.WeaponInventory` _playerref_4)) 1))
        (set `/Game/Others/FPS_System/Game/Blueprints/Player_BP.WeaponIndex` 0 _playerref)
        (else
          (set `/Game/Others/FPS_System/Game/Blueprints/Player_BP.WeaponIndex` _returnvalue _playerref))))
    (:`then_1`
      (if (!= (`/Game/Others/FPS_System/Game/Blueprints/Player_BP.WeaponIndex` _playerref_4) 1)
        ;;[1 1 1] Primary to Secondary
        (bind _output_get (set `self.SwitchEnd` (`self.SwitchEnd`)))
        (`|PlayMontage` _mesh _output_get
          (:`OnBlendOut`
            _)
          (:`OnInterrupted`
            _))
        (`self.K2_AttachToComponent` (`/Game/Others/FPS_System/Game/Blueprints/Player_BP.EquippedWeapon` (`self.PlayerRef`)) _mesh "Secondary_Holster" "SnapToTarget" "SnapToTarget" "KeepRelative" true)
        (`self.K2_AttachToComponent` _output _mesh "Weapon_Point" "SnapToTarget" "SnapToTarget" "KeepRelative" true)
        (`|ExecutionSequence`
          (:`then_0`
            (`KismetSystemLibrary.Delay` 2.0)
            (set `self.IsSwitching` false))
          (:`then_1`
            (set `/Game/Others/FPS_System/Game/Blueprints/Player_BP.EquippedWeapon` _output (`self.PlayerRef`))
            (bind _output_get_2 (set `self.SwitchStart` (`self.SwitchStart`)))
            (`|PlayMontage` _mesh _output_get_2)))
        (else
          ;;[1 1 1] Secondary to Primary
          (bind _output_get_3 (set `self.SwitchEnd` (`self.SwitchEnd`)))
          (`|PlayMontage` _mesh _output_get_3
            (:`OnBlendOut`
              _)
            (:`OnInterrupted`
              _))
          (`self.K2_AttachToComponent` (`/Game/Others/FPS_System/Game/Blueprints/Player_BP.EquippedWeapon` (`self.PlayerRef`)) _mesh "Primary_Holster_2" "SnapToTarget" "SnapToTarget" "KeepRelative" true)
          (`self.K2_AttachToComponent` _output_2 _mesh "Weapon_Point" "SnapToTarget" "SnapToTarget" "KeepRelative" true)
          (`|ExecutionSequence`
            (:`then_0`
              (`KismetSystemLibrary.Delay` 2.0)
              (set `self.IsSwitching` false))
            (:`then_1`
              (set `/Game/Others/FPS_System/Game/Blueprints/Player_BP.EquippedWeapon` _output_2 (`self.PlayerRef`))
              (bind _output_get_4 (set `self.SwitchStart` (`self.SwitchStart`)))
              (`|PlayMontage` _mesh _output_get_4))))))))

(fn `Projectile`
  (bind _returnvalue (`KismetMathLibrary.RandomFloatInRange` 0.2 0.4))
  (bind _weaponmesh (`self.WeaponMesh`))
  (bind _returnvalue_2 (`SceneComponent.GetSocketLocation` _weaponmesh "Shell_Eject"))
  (bind _returnvalue_3 (`SceneComponent.GetSocketRotation` _weaponmesh "Muzzle"))
  (bind _returnvalue_4 (`SceneComponent.GetSocketLocation` _weaponmesh "Muzzle"))
  (bind _returnvalue_5 (* (`KismetMathLibrary.VSize` (`KismetMathLibrary.ClampVectorSize` (`self.GetVelocity`) 0.0 1.0)) (`KismetMathLibrary.RandomFloatInRange` -1000.0 1000.0)))
  ;[1 1 1] Shot Offset
  (bind _asplayer_bp (cast `/Game/Others/FPS_System/Game/Blueprints/Player_BP` (`GameplayStatics.GetPlayerCharacter` 0)))
  (`Pawn.AddControllerPitchInput` _asplayer_bp (`KismetMathLibrary.RandomFloatInRange` -0.8 -1.0))
  (`Pawn.AddControllerYawInput` _asplayer_bp (`KismetMathLibrary.RandomFloatInRange` -0.3 0.3))
  (`GameplayStatics.SpawnEmitterAttached` "/Game/Others/FPS_System/Game/Weapons/Commons/Particles/P_MuzzleFlash.P_MuzzleFlash" _weaponmesh "Muzzle" _returnvalue_4 _returnvalue_3 (1.0 1.0 1.0) "KeepWorldPosition")
  (`GameplayStatics.SpawnEmitterAttached` "/Game/Others/FPS_System/Game/Weapons/Commons/Particles/P_Shells.P_Shells" _weaponmesh "Shell_Eject" _returnvalue_2 (`SceneComponent.GetSocketRotation` _weaponmesh "Shell_Eject") (1.0 1.0 1.0) "KeepWorldPosition")
  (`|ExecutionSequence`
    (:`then_0`
      (`GameplayStatics.PlaySoundAtLocation` (`.FireSound_63_8052C813477A4A0B355FEA8677AC9B05` (break `/Game/Others/FPS_System/Game/Blueprints/Weapon_Struct` (`self.WeaponData`))) _returnvalue_2 (struct) 1.0 1.0 0.0 null null null)
      (`GameplayStatics.PlaySoundAtLocation` "/Game/Others/FPS_System/Game/Sounds/Wave/Shell.Shell" _returnvalue_2 (struct) _returnvalue 0.98 _returnvalue null null null)
      (bind _fpcamera (`/Game/Others/FPS_System/Game/Blueprints/Player_BP.FPCamera` _asplayer_bp))
      (bind _returnvalue_6 (`SceneComponent.K2_GetComponentLocation` _fpcamera))
      (bind (_outhit _returnvalue_7) (`KismetSystemLibrary.LineTraceSingle` _returnvalue_6 (+ _returnvalue_6 (* (`SceneComponent.GetForwardVector` _fpcamera) 500000.0) (`KismetMathLibrary.MakeVector` _returnvalue_5 _returnvalue_5 _returnvalue_5)) "TraceTypeQuery1"))
      (`|SpawnActorFromClass` "/Game/Others/FPS_System/Game/Blueprints/Bullet_Projectile.Bullet_Projectile_C" (`KismetMathLibrary.MakeTransform` _returnvalue_4 _returnvalue_3) "Undefined" "OverrideRootScale" null null)
      (if _returnvalue_7
        (bind (_bblockinghit _binitialoverlap _time _distance _location _impactpoint _normal _impactnormal) (`GameplayStatics.BreakHitResult` _outhit))
        ;[1 1 1] At Impact
        (`GameplayStatics.PlaySoundAtLocation` "/Game/Others/FPS_System/Game/Sounds/Wave/SMG_Fire_Single.SMG_Fire_Single" _impactpoint (struct) 0.1 200.0 0.0 null null null)
        (`GameplayStatics.SpawnEmitterAtLocation` "/Game/Others/FPS_System/Game/Weapons/Commons/Particles/P_ImpactHit.P_ImpactHit" _impactpoint (`KismetMathLibrary.Conv_VectorToRotator` _normal))
        (`|SpawnActorFromClass` "/Game/Others/FPS_System/Game/Weapons/Commons/Particles/Materials/Decals/Bullet_Hole.Bullet_Hole_C" (`KismetMathLibrary.MakeTransform` _location (`KismetMathLibrary.Conv_VectorToRotator` _impactnormal)) "Undefined" "OverrideRootScale" null null)))
    (:`then_1`
      (`GameplayStatics.PlayWorldCameraShake` "/Game/Others/FPS_System/Game/Blueprints/Headbobbing/ShootShake.ShootShake_C" (`self.K2_GetActorLocation`) 0.0 200.0))))

(fn `UserConstructionScript`
  (bind (_weapondata_class _weapondata_name _weapondata_firerate _weapondata_firemodes _weapondata_defaultfm _weapondata_magazinesize _weapondata_currentammo _weapondata_maxammo _weapondata_holsterslot _weapondata_reloadshort_length _weapondata_reloadlong_length _weapondata_firesound) (break `/Game/Others/FPS_System/Game/Blueprints/Weapon_Struct` (`self.WeaponData`)))
  (set `self.WeaponData` (make `/Game/Others/FPS_System/Game/Blueprints/Weapon_Struct` _weapondata_class _weapondata_name _weapondata_firerate _weapondata_firemodes _weapondata_defaultfm _weapondata_magazinesize _weapondata_currentammo _weapondata_maxammo _weapondata_holsterslot _weapondata_reloadshort_length _weapondata_reloadlong_length _weapondata_firesound)))