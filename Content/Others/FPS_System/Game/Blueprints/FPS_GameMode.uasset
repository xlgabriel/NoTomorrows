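; FPS game mode that randomizes which killable Blind Folk characters remain in the level when play begins.
; On BeginPlay it gathers every BlindFolkCrctrKillable actor, shuffles the array and destroys the surplus, leaving a random subset sized by BlinkFolksKillablesInMap.
; It decrements the total killable count for each removal and resets the remaining-killables counter to zero within the same loop.
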(event `self.ReceiveBeginPlay`
  (`|ExecutionSequence`
    (:`then_0`
      (bind _outactors (`GameplayStatics.GetAllActorsOfClass` "/Game/HorrorTemplate/Enemigo/BlindFolk/BlinkFolkKillable/BlindFolkCrctrKillable.BlindFolkCrctrKillable_C"))
      (`KismetArrayLibrary.Array_Shuffle` _outactors)
      (bind _returnvalue (`KismetArrayLibrary.Array_Length` _outactors))
      (set `self.TotalBlinkFolksKillables` _returnvalue)
      (for _index (range (+ (- _returnvalue (+ (`self.BlinkFolksKillablesInMap`) 1)) 1))
        (`self.K2_DestroyActor` (`|GetArrayItem` _outactors _index))
        (set `self.TotalBlinkFolksKillables` (- (`self.TotalBlinkFolksKillables`) 1))
        (set `self.BlinkFolksKillablesLeft` 0)))))

(fn `UserConstructionScript`)