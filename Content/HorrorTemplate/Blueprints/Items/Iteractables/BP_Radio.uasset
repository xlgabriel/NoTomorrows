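; BP_Radio is an interactable radio item from the horror template that can be switched on and off.
; Its construction script runs the parent's, assigns the configurable Sound to the Audio component and toggles that component's active state if StartOn is set.
; The Use event toggles the Audio component and plays UseSound at the Cube component's location as feedback.
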(event `self.Use`
  (params (MiscUse1 :type Boolean))
  ;[1 1 1] Play sound at location
  (`ActorComponent.ToggleActive` (`self.Audio`))
  (`GameplayStatics.PlaySoundAtLocation` (`self.UseSound`) (`SceneComponent.K2_GetComponentLocation` (`self.Cube`))))

(fn `UserConstructionScript`
  (bind _audio (`self.Audio`))
  (`parent.UserConstructionScript`)
  (`AudioComponent.SetSound` _audio (`self.Sound`))
  (if (`self.StartOn`)
    (`ActorComponent.ToggleActive` _audio)))