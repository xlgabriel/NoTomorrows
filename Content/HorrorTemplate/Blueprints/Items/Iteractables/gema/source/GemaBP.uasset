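; GemaBP is a collectible gem that the player picks up with the Use input while standing inside its capsule.
; Capsule overlap with the HorrorTemplateCharacter enables input on the actor, and leaving the capsule disables it.
; On Use, it decrements GemsLeft in HorrorTemplateGamemode, adds a new GemWidget to the viewport, plays a pickup sound and destroys itself.
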(event `InputAction|Use`
  (params (Key :type "Key Structure"))
  (:`Pressed`
    (bind _ashorror_template_gamemode (cast `/Game/HorrorTemplate/Blueprints/Character/HorrorTemplateGamemode` (`GameplayStatics.GetGameMode`)))
    (bind _result (`/Engine/EditorBlueprintResources/StandardMacros.DecrementInt` (`/Game/HorrorTemplate/Blueprints/Character/HorrorTemplateGamemode.GemsLeft` _ashorror_template_gamemode))
      (:`  `
        (set `/Game/HorrorTemplate/Blueprints/Character/HorrorTemplateGamemode.GemsLeft` _result _ashorror_template_gamemode)
        (bind _returnvalue (`|CreateWidget` "/Game/HorrorTemplate/Blueprints/Items/Iteractables/gema/source/GemWidget.GemWidget_C"))
        (`UserWidget.AddToViewport` _returnvalue 0)
        (`GameplayStatics.PlaySoundAtLocation` "/Game/HorrorTemplate/Blueprints/Items/Iteractables/gema/gemsound.gemsound" (`self.K2_GetActorLocation`) (struct) 0.5 1.0 0.0 null null null)
        (`self.K2_DestroyActor`)))))

(event `self.Capsule.OnComponentBeginOverlap`
  (params (OverlappedComponent :type "PrimitiveComponent Object Reference") (OtherActor :type "Actor Object Reference") (OtherComp :type "PrimitiveComponent Object Reference") (OtherBodyIndex :type Integer) (bFromSweep :type Boolean) (SweepResult :type "HitResult Structure (by ref)"))
  (cast `/Game/HorrorTemplate/Blueprints/Character/HorrorTemplateCharacter` OtherActor)
  (`self.EnableInput` (`GameplayStatics.GetPlayerController` 0)))

(event `self.Capsule.OnComponentEndOverlap`
  (params (OverlappedComponent :type "PrimitiveComponent Object Reference") (OtherActor :type "Actor Object Reference") (OtherComp :type "PrimitiveComponent Object Reference") (OtherBodyIndex :type Integer))
  (cast `/Game/HorrorTemplate/Blueprints/Character/HorrorTemplateCharacter` OtherActor)
  (`self.DisableInput` (`GameplayStatics.GetPlayerController` 0)))

(fn `UserConstructionScript`)