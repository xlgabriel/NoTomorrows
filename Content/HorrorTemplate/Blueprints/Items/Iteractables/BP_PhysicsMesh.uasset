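; Physics prop actor with a configurable mesh and mass that plays impact sounds when it collides.
; It simulates physics from the start if StartAwake is set, otherwise it stays still until a hit turns simulation on.
; On hit, the impulse is remapped against mass, and results above a mass-scaled threshold play an attenuated sound with clamped, impulse-based volume.
; A short retriggerable delay on CanHit prevents sound spam.
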(event `self.ReceiveBeginPlay`
  (bind _staticmesh (`self.StaticMesh`))
  ;[1 1 1] If starts asleep, then disable simulate physics
  (if (`self.StartAwake`)
    (`PrimitiveComponent.SetSimulatePhysics` _staticmesh true)
    (else
      (`PrimitiveComponent.SetSimulatePhysics` _staticmesh false))))

(event `self.ReceiveHit`
  (params (MyComp :type "PrimitiveComponent Object Reference") (Other :type "Actor Object Reference") (OtherComp :type "PrimitiveComponent Object Reference") (bSelfMoved :type Boolean) (HitLocation :type "Vector Structure") (HitNormal :type "Vector Structure") (NormalImpulse :type "Vector Structure") (Hit :type "HitResult Structure (by ref)"))
  (bind _returnvalue (`PrimitiveComponent.GetMass` (`self.StaticMesh`)))
  (bind _returnvalue_2 (* _returnvalue 10.0))
  (bind _returnvalue_3 (`KismetMathLibrary.VSize` (`KismetMathLibrary.MakeVector` (`KismetMathLibrary.MapRangeClamped` (.x NormalImpulse) 0.0 25000.0 0.0 _returnvalue_2) (`KismetMathLibrary.MapRangeClamped` (.y NormalImpulse) 0.0 25000.0 0.0 _returnvalue_2) (`KismetMathLibrary.MapRangeClamped` (.z NormalImpulse) 0.0 25000.0 0.0 _returnvalue_2))))
  ;[1 1 1] Impact Sounds
  (if (`self.CanHit`)
    ;;[1 1 1] If bumped into, then simulate physics
    (if (not (`self.StartAwake`))
      (`PrimitiveComponent.SetSimulatePhysics` (`self.StaticMesh`) true))
    ;;[1 1 1] If impulse length is greater than impact threshold then play impact sound
    (if (>= _returnvalue_3 (* (`self.ImpactThresholdMultiplier`) _returnvalue))
      (`GameplayStatics.PlaySoundAtLocation` (`self.ImpactSound`) HitLocation (struct) (`KismetMathLibrary.FClamp` _returnvalue_3 0.25 2.0) (`self.PitchMultiplier`) 0.0 "/Game/HorrorTemplate/Sounds/Attenuation/ATT_PhysicsImpact.ATT_PhysicsImpact")
      ;;[1 1 1] Prevent too many sounds playing too soon
      (set `self.CanHit` false)
      (`KismetSystemLibrary.RetriggerableDelay` 0.2)
      (set `self.CanHit` true))))

(fn `UserConstructionScript`
  (bind _staticmesh (`self.StaticMesh`))
  (`StaticMeshComponent.SetStaticMesh` _staticmesh (`self.Static Mesh`))
  ;[1 1 1] Set custom mass
  (`PrimitiveComponent.SetMassOverrideInKg` _staticmesh "None" (`self.Mass`) true))