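; BP_Ladder is a climbable ladder for the horror template, built from a trigger box and a cube ladder mesh.
; On overlap it switches the HorrorTemplateCharacter to Flying movement as a hacky climb and sets IsOnLadder, then restores Walking on exit.
; The construction script optionally applies a custom trigger height and, when ShowLadder is off, toggles the cube's visibility and disables its collision.
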(event `self.ReceiveActorBeginOverlap`
  (params (OtherActor :type "Actor Object Reference"))
  ;[1 1 1] Set the players movement to flying to simulate being able to move vertically, very hacky
  (bind _ashorror_template_character (cast `/Game/HorrorTemplate/Blueprints/Character/HorrorTemplateCharacter` OtherActor)
    (:`then`
      (`CharacterMovementComponent.SetMovementMode` (`Character.CharacterMovement` _ashorror_template_character) "MOVE_Flying" 0)
      (set `/Game/HorrorTemplate/Blueprints/Character/HorrorTemplateCharacter.IsOnLadder` true _ashorror_template_character))
    (:`CastFailed`
      ;[1 1 1] Fail Event
      (`KismetSystemLibrary.PrintString` "PLAYER OVERLAP CAST FALED" true true (struct :`R` 1.0 :`A` 1.0) :!label _label))))

(event `self.ReceiveActorEndOverlap`
  (params (OtherActor :type "Actor Object Reference"))
  ;[1 1 1] Set movement back to walking
  (bind _ashorror_template_character (cast `/Game/HorrorTemplate/Blueprints/Character/HorrorTemplateCharacter` OtherActor)
    (:`then`
      (`CharacterMovementComponent.SetMovementMode` (`Character.CharacterMovement` _ashorror_template_character) "MOVE_Walking" 0)
      (set `/Game/HorrorTemplate/Blueprints/Character/HorrorTemplateCharacter.IsOnLadder` false _ashorror_template_character))
    (:`CastFailed`
      (goto _label))))

(fn `UserConstructionScript`
  (bind _cube (`self.Cube`))
  ;[1 1 1] Set trigger extents
  (if (`self.UseCustomHeight`)
    (`BoxComponent.SetBoxExtent` (`self.Box`) (`KismetMathLibrary.MakeVector` 32.0 25.0 (`self.Height`)) true))
  (if (`self.ShowLadder`)
    ;[1 1 1] Disable cube ladder collision
    (`PrimitiveComponent.SetCollisionEnabled` _cube "QueryAndPhysics")
    (else
      (`/Engine/EditorBlueprintResources/StandardMacros.FlipFlop`
        (:`A`
          _)
        (:`B`
          _))
      ;[1 1 1] Should show cube ladder or not
      (`SceneComponent.ToggleVisibility` _cube false)
      (`PrimitiveComponent.SetCollisionEnabled` (`self.Cube`) "NoCollision"))))