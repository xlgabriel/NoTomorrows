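; Readable note pickup for the horror template that shows its image on the player's HUD.
; Box overlaps set the character's HasNote flag, and leaving also removes a displayed note.
; Use alternates via FlipFlop between DisplayNote, which sets the HUD brush and plays a sound if HasNote is true, and RemoveNote.
; The construction script sizes the trigger and applies the note texture through a dynamic material instance.
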(event `self.ReceiveActorBeginOverlap`
  (params (OtherActor :type "Actor Object Reference"))
  ;[1 1 1] Only allow us to use the note if we are within the trigger bounds
  (if (== (`GameplayStatics.GetObjectClass` OtherActor) (`GameMode.DefaultPawnClass` (`GameplayStatics.GetGameMode`)))
    (bind _ashorror_template_character (cast `/Game/HorrorTemplate/Blueprints/Character/HorrorTemplateCharacter` (`GameplayStatics.GetPlayerCharacter` 0))
      (:`then`
        (set `/Game/HorrorTemplate/Blueprints/Character/HorrorTemplateCharacter.HasNote` true _ashorror_template_character))
      (:`CastFailed`
        ;;[1 1 1] Fail Event
        (`KismetSystemLibrary.PrintString` "PLAYER CAST FALED" true true (struct :`R` 1.0 :`A` 1.0))))))

(event `self.ReceiveActorEndOverlap`
  (params (OtherActor :type "Actor Object Reference"))
  ;[1 1 1] We are outside the trigger bounds, so remove the note from our screen
  (if (== (`GameplayStatics.GetObjectClass` OtherActor) (`GameMode.DefaultPawnClass` (`GameplayStatics.GetGameMode`)))
    (bind _ashorror_template_character (cast `/Game/HorrorTemplate/Blueprints/Character/HorrorTemplateCharacter` (`GameplayStatics.GetPlayerCharacter` 0))
      (:`then`
        (set `/Game/HorrorTemplate/Blueprints/Character/HorrorTemplateCharacter.HasNote` false _ashorror_template_character)
        (if (`/Game/HorrorTemplate/Blueprints/Character/HorrorTemplateCharacter.IsNoteDisplayed` _ashorror_template_character)
          (`/Game/HorrorTemplate/Blueprints/Character/HorrorTemplateCharacter.RemoveNote` _ashorror_template_character)))
      (:`CastFailed`
        ;[1 1 1] Fail Event
        (`KismetSystemLibrary.PrintString` "PLAYER CAST FALED" true true (struct :`R` 1.0 :`A` 1.0))))))

(event `self.Use`
  (params (MiscUse1 :type Boolean))
  (bind _ashorror_template_character (cast `/Game/HorrorTemplate/Blueprints/Character/HorrorTemplateCharacter` (`GameplayStatics.GetPlayerCharacter` 0))
    (:`then`
      ;[1 1 1] Display the note one the players HUD
      (`/Engine/EditorBlueprintResources/StandardMacros.FlipFlop`
        (:`A`
          (`self.DisplayNote`))
        (:`B`
          (`/Game/HorrorTemplate/Blueprints/Character/HorrorTemplateCharacter.RemoveNote` _ashorror_template_character))))
    (:`CastFailed`
      ;[1 1 1] Fail Event
      (`KismetSystemLibrary.PrintString` "PLAYER CAST FALED" true true (struct :`R` 1.0 :`A` 1.0)))))

(fn `DisplayNote`
  (bind _ashorror_template_character (cast `/Game/HorrorTemplate/Blueprints/Character/HorrorTemplateCharacter` (`GameplayStatics.GetPlayerCharacter` 0))
    (:`then`
      ;[1 1 1] Change note texture on hud to that of this note
      (set `/Game/HorrorTemplate/Blueprints/Character/HUD/Hud_Note.NoteImageBrush` (`self.NoteImage`) (`/Game/HorrorTemplate/Blueprints/Character/HorrorTemplateCharacter.Hud_Note` _ashorror_template_character))
      ;[1 1 1] If player has note, then display it and play a sound
      (if (`/Game/HorrorTemplate/Blueprints/Character/HorrorTemplateCharacter.HasNote` _ashorror_template_character)
        (`/Game/HorrorTemplate/Blueprints/Character/HorrorTemplateCharacter.DisplayNote` _ashorror_template_character)
        (`GameplayStatics.PlaySound2D` (`self.NoteSound`))))
    (:`CastFailed`
      ;[1 1 1] Fail Event
      (`KismetSystemLibrary.PrintString` "PLAYER CAST FALED" true true (struct :`R` 1.0 :`A` 1.0)))))

(fn `UserConstructionScript`
  (`parent.UserConstructionScript`)
  (`BoxComponent.SetBoxExtent` (`self.Box`) (`self.TriggerExtents`) true)
  ;[1 1 1] All us to edit the material instance
  (bind _returnvalue (`PrimitiveComponent.CreateDynamicMaterialInstance` (`self.StaticMesh`) 0 "/Game/HorrorTemplate/Materials/Items/Notes/Mat_note.Mat_note"))
  ;[1 1 1] Allows you to change the material to use the texture
  (`MaterialInstanceDynamic.SetTextureParameterValue` _returnvalue "NoteTexture" (`self.NoteTexture`)))