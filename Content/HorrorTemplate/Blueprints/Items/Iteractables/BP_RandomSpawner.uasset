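; BP_RandomSpawner is a horror template Blueprint that spawns a configurable ActorToSpawn at randomly picked locations on BeginPlay.
; A loop with a random count reads transforms from the SpawnActor array, intended to hold child actors, and removes entries as it goes.
; Separate random index picks for validation, spawning and removal can hit different entries, and the author's comment flags the spawner as buggy.
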(event `self.ReceiveBeginPlay`
  (bind _spawnactor (`self.SpawnActor`))
  (bind _returnvalue (`KismetMathLibrary.RandomIntegerInRange` 0 (- (`KismetArrayLibrary.Array_Length` _spawnactor) 1)))
  (bind _item (`KismetArrayLibrary.Array_Get` (`self.SpawnActor`) _returnvalue))
  ;[1 1 1] Buggy random spawner, use child actors as spawn locations
  ;;[1 1 1] Repeat until finished
  (for _ (range (+ _returnvalue 1))
    (`/Engine/EditorBlueprintResources/StandardMacros.IsValid` _item
      (:`Is Valid`
        ;;[1 1 1] Spawn whatever item
        (`|SpawnActorFromClass` (`self.ActorToSpawn`) (`self.GetTransform` _item) "Undefined" "OverrideRootScale")
        (`KismetArrayLibrary.Array_Remove` _spawnactor _returnvalue))
      (:`Is Not Valid`
        (break)))))

(fn `UserConstructionScript`
  (`parent.UserConstructionScript`))