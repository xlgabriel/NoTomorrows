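; Two-panel interactable sliding door for the horror template that toggles open and closed on each Use event.
; A FlipFlop plays or reverses the DoorMove timeline, which lerps both panels apart along local Y from relative positions cached in the construction script.
; Each use plays the open sound and a camera shake centred on the left panel's cached relative location; timeline completion plays the close sound.
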(event `self.Use`
  (params (MiscUse1 :type Boolean))
  (bind _rightdoorinitiallocation (`self.RightDoorInitialLocation`))
  (bind _leftdoorinitiallocation (`self.LeftDoorInitialLocation`))
  ;[1 1 1] Open Sound
  (`GameplayStatics.PlaySoundAtLocation` (`self.OpenSound`) (`SceneComponent.K2_GetComponentLocation` (`self.LeftDoor`)) (struct) (`self.OpenVolume`) 0.7 0.0 "/Game/HorrorTemplate/Sounds/Attenuation/ATT_Door.ATT_Door")
  ;[1 1 1] Shake camera when opening door
  (`GameplayStatics.PlayWorldCameraShake` "/Game/HorrorTemplate/Blueprints/Items/Effects/CS_Door.CS_Door_C" (`self.LeftDoorInitialLocation`) 0.0 500.0 0.0)
  (`/Engine/EditorBlueprintResources/StandardMacros.FlipFlop`
    (:`A`
      ;[1 1 1] Set door move locations, and lerp between them
      (bind (_direction _newtrack_0) (`Timeline|DoorMove` :!label _label)
        (:`Update`
          (`SceneComponent.K2_SetRelativeLocation` (`self.LeftDoor`) (`KismetMathLibrary.VLerp` _leftdoorinitiallocation (- _leftdoorinitiallocation (-0.0 90.0 0.0)) _newtrack_0) false false)
          (`SceneComponent.K2_SetRelativeLocation` (`self.RightDoor`) (`KismetMathLibrary.VLerp` _rightdoorinitiallocation (- _rightdoorinitiallocation (-0.0 -90.0 0.0)) _newtrack_0) false false))
        (:`Finished`
          ;[1 1 1] Close Sound
          (`GameplayStatics.PlaySoundAtLocation` (`self.CloseSound`) (`SceneComponent.K2_GetComponentLocation` (`self.RightDoor`)) (struct) (`self.CloseVolume`) 1.0 0.0 "/Game/HorrorTemplate/Sounds/Attenuation/ATT_Door.ATT_Door"))))
    (:`B`
      (goto _label :!via `Reverse`))))

(fn `UserConstructionScript`
  ;[1 1 1] Set door locations
  (`parent.UserConstructionScript`)
  (set `self.LeftDoorInitialLocation` (`SceneComponent.RelativeLocation` (`self.LeftDoor`)))
  (set `self.RightDoorInitialLocation` (`SceneComponent.RelativeLocation` (`self.RightDoor`))))