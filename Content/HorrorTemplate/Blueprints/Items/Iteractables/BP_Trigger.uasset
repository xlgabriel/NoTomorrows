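; BP_Trigger is a placeable box trigger that activates linked interactables when an actor overlaps it.
; On overlap it loops over its OtherActor array, casts each entry to BP_Interactable and calls Use with ShouldUnlock, printing a message on failed casts.
; FireOnce limits it to a single activation through HasFired, which is set only after a successful cast.
; The construction script sizes the box from TriggerExtents.
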(event `self.ReceiveActorBeginOverlap`
  (params (OtherActor :type "Actor Object Reference"))
  ;[1 1 1] If fire once, then dont repeat
  (if (`self.FireOnce`)
    (if (not (`self.HasFired`))
      ;[1 1 1] Repeat for how many ever actors selected
      (for _array_element (`self.OtherActor`) :!label _label
        ;[1 1 1] Use function to unlock or do something
        (bind _asbp_interactable (cast `/Game/HorrorTemplate/Blueprints/Items/Iteractables/BP_Interactable` _array_element)
          (:`then`
            (`self.Use` _asbp_interactable (`self.ShouldUnlock`))
            (set `self.HasFired` true))
          (:`CastFailed`
            ;[1 1 1] Fail Event
            (`KismetSystemLibrary.PrintString` "INTERACTABLE CAST FAILED" true true (struct :`R` 1.0 :`A` 1.0))))))
    (else
      (goto _label))))

(fn `UserConstructionScript`
  (`parent.UserConstructionScript`)
  ;[1 1 1] Set trigger extents
  (`BoxComponent.SetBoxExtent` (`self.Box`) (`self.TriggerExtents`) true))