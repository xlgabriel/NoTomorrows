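; Horror template game mode that randomizes how many blind folk characters and batteries populate the map when play begins.
; BeginPlay shuffles the placed actors of each type and destroys the surplus, so a random subset matching the configured in-map count remains.
; It records the remaining totals, zeroes their "Left" counters when culling, and counts all gems as both total and left without removing any.
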(event `self.ReceiveBeginPlay`
  (`|ExecutionSequence`
    (:`then_0`
      (bind _outactors (`GameplayStatics.GetAllActorsOfClass` "/Game/HorrorTemplate/Enemigos/BlindFolk/BlindFolkCrctr.BlindFolkCrctr_C"))
      (`KismetArrayLibrary.Array_Shuffle` _outactors)
      (bind _returnvalue (`KismetArrayLibrary.Array_Length` _outactors))
      (set `self.TotalBlinkFolks` _returnvalue)
      (for _index (range (+ (- _returnvalue (+ (`self.BlinkFolksInMap`) 1)) 1))
        (`self.K2_DestroyActor` (`|GetArrayItem` _outactors _index))
        (set `self.TotalBlinkFolks` (- (`self.TotalBlinkFolks`) 1))
        (set `self.BlinkFolksLeft` 0)))
    (:`then_1`
      (bind _outactors_2 (`GameplayStatics.GetAllActorsOfClass` "/Game/HorrorTemplate/Blueprints/Items/Iteractables/BP_Battery.BP_Battery_C"))
      (`KismetArrayLibrary.Array_Shuffle` _outactors_2)
      (bind _returnvalue_2 (`KismetArrayLibrary.Array_Length` _outactors_2))
      (set `self.TotalBatteries` _returnvalue_2)
      (for _index_2 (range (+ (- _returnvalue_2 (+ (`self.BatteriesInMap`) 1)) 1))
        (`self.K2_DestroyActor` (`|GetArrayItem` _outactors_2 _index_2))
        (set `self.TotalBatteries` (- (`self.TotalBatteries`) 1))
        (set `self.BatteriesLeft` 0)))
    (:`then_2`
      (bind _outactors_3 (`GameplayStatics.GetAllActorsOfClass` "/Game/HorrorTemplate/Blueprints/Items/Iteractables/gema/source/GemaBP.GemaBP_C"))
      (bind _output_get (set `self.GemsLeft` (`KismetArrayLibrary.Array_Length` _outactors_3)))
      (set `self.TotalGems` _output_get))))

(fn `UserConstructionScript`)